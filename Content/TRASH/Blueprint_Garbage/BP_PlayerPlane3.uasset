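; Prototype player plane that flies in a straight line along a Direction vector at a set Speed.
; Tick offsets the StaticMesh world location by normalized Direction, Speed and delta time, then sets the actor transform with zero rotation and no sweep.
; The Yaw axis adds rate-scaled controller yaw input, which does not feed Direction.
; An A key handler increments TESTVAR as an input test independent of Tick.
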(event EventBeginPlay)

(event Collision|EventActorBeginOverlap
  (params (OtherActor :type Actor%20Object%20Reference)))

(event EventTick
  (params (DeltaSeconds :type Float%20%28single-precision%29))
  (bind _staticmesh (Variables|Default|GetStaticMesh))
  (bind _returnvalue (Transformation|GetWorldTransform _staticmesh))
  (bind (_location _rotation _scale) (Math|Transform|BreakTransform _returnvalue))
  (Transformation|SetActorTransform (Math|Transform|MakeTransform (+ (* (Math|Vector|Normalize (Variables|Default|GetDirection)) (* (Utilities|Time|GetWorldDeltaSeconds) (Variables|Default|GetSpeed))) _location) "0, 0, 0" _scale)))

(event Input|AxisEvents|InputAxisYaw
  (params (AxisValue :type Float%20%28single-precision%29))
  (Pawn|Input|AddControllerYawInput (* AxisValue (Variables|Default|GetTurn%20Rate) (Utilities|Time|GetWorldDeltaSeconds))))

(event Input|KeyboardEvents|A
  (params (Key :type Key%20Structure))
  ;[1 1 1] PROOF THAT INPUT DOESN'T NEED TO BE HOOKED TO EVENT TICK
  (:Pressed
    (if true
      (Variables|Default|SetTEST%20VAR (+ (Variables|Default|GetTEST%20VAR) 1e+01))
      (else
        (Variables|Default|SetTEST%20VAR 0.0)))))

(fn ConstructionScript)