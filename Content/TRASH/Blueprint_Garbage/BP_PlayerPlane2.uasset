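; BP_PlayerPlane2 is an actor that shows a configurable static mesh and drives a rotating movement component.
; The construction script applies the Mesh variable to StaticMesh and copies rotation rate, pivot translation and local-space settings into RotatingMovement.
; At BeginPlay, RotatingMovement is pointed at the Cube component as its updated component.
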(event EventBeginPlay
  (Components|Movement|SetUpdatedComponent (Variables|Default|GetRotatingMovement) (Variables|Default|GetCube)))

(event Collision|EventActorBeginOverlap
  (params (OtherActor :type Actor%20Object%20Reference)))

(fn ConstructionScript
  (bind _rotatingmovement (Variables|Default|GetRotatingMovement))
  (Components|StaticMesh|SetStaticMesh (Variables|Default|GetStaticMesh) (Variables|Default|GetMesh))
  (Variables|/Script/Engine.RotatingMovementComponent|SetRotationRate _rotatingmovement (Variables|Default|GetRotation%20Rate))
  (Variables|/Script/Engine.RotatingMovementComponent|SetPivotTranslation _rotatingmovement (Variables|Default|GetPivot%20Translation))
  (Variables|/Script/Engine.RotatingMovementComponent|SetbRotationInLocalSpace _rotatingmovement (Variables|Default|GetRotation%20in%20Local%20Space)))