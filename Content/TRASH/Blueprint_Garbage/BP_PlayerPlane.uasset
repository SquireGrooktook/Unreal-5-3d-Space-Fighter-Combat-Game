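; BP_PlayerPlane is an actor Blueprint for a player plane that moves continuously in a straight line along its Direction variable.
; Each Tick it scales the normalized Direction by Speed and world delta time, then adds that to the StaticMesh's world location.
; It sets the actor transform without sweeping, zeroing rotation and reusing the mesh's world scale.
; The graph has no input handling, and BeginPlay, overlap and construction logic are empty.
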(event EventBeginPlay)

(event Collision|EventActorBeginOverlap
  (params (OtherActor :type Actor%20Object%20Reference)))

(event EventTick
  (params (DeltaSeconds :type Float%20%28single-precision%29))
  (bind _staticmesh (Variables|Default|GetStaticMesh))
  (bind _returnvalue (Transformation|GetWorldTransform _staticmesh))
  (bind (_location _rotation _scale) (Math|Transform|BreakTransform _returnvalue))
  (Transformation|SetActorTransform (Math|Transform|MakeTransform (+ (* (Math|Vector|Normalize (Variables|Default|GetDirection)) (* (Utilities|Time|GetWorldDeltaSeconds) (Variables|Default|GetSpeed))) _location) "0, 0, 0" _scale)))

(event Input|KeyboardEvents|A
  (params (Key :type Key%20Structure)))

(event Input|KeyboardEvents|D
  (params (Key :type Key%20Structure)))

(fn ConstructionScript)