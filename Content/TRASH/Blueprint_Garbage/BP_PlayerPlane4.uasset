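; Player-controlled plane that flies constantly along its static mesh's forward vector, with steering, speed control and projectile fire.
; Tick moves the actor and re-arms firing through a FireRate Delay.
; Pitch and Yaw inputs share one mesh rotation update and also shift spring-arm lengths for clamped, self-recentering camera offsets.
; Roll input selects fast, slow or default speed, and fire input spawns BP_ProjectileActor1 along the mesh rotation.
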(event EventTick
  (params (DeltaSeconds :type Float%20%28single-precision%29))
  (bind _staticmesh (Variables|Default|GetStaticMesh))
  (bind _returnvalue (Transformation|GetWorldTransform _staticmesh))
  (bind (_location _rotation _scale) (Math|Transform|BreakTransform _returnvalue))
  (Transformation|SetActorTransform (Math|Transform|MakeTransform (+ (* (Math|Vector|Normalize (Math|Vector|GetForwardVector _staticmesh)) (* (Utilities|Time|GetWorldDeltaSeconds) (Variables|Default|GetMovement%20Speed))) _location) "0, 0, 0" _scale))
  (Utilities|FlowControl|Delay (Variables|Default|GetFire%20Rate))
  (Variables|Default|SetFire%20Okay true))

(event Input|AxisEvents|InputAxisPitch
  (params (AxisValue :type Float%20%28single-precision%29))
  (bind _staticmesh (Variables|Default|GetStaticMesh))
  (bind _returnvalue (Transformation|GetWorldRotation _staticmesh))
  ;[1 1 1] Comment
  (Transformation|SetWorldRotation _staticmesh (Math|Rotator|MakeRotator 0.0 (+ (* AxisValue (Variables|Default|GetTurn%20Rate) (Utilities|Time|GetWorldDeltaSeconds)) (.pitch _returnvalue)) (+ (* (stale Input|AxisEvents|InputAxisYaw AxisValue) (Variables|Default|GetTurn%20Rate) (Utilities|Time|GetWorldDeltaSeconds)) (.yaw _returnvalue))) false false))

(event Input|AxisEvents|InputAxisYaw
  (params (AxisValue :type Float%20%28single-precision%29))
  (bind _staticmesh (Variables|Default|GetStaticMesh))
  (bind _returnvalue (Transformation|GetWorldRotation _staticmesh))
  ;[1 1 1] This is the left/right one...
  (Transformation|SetWorldRotation _staticmesh (Math|Rotator|MakeRotator 0.0 (+ (* (stale Input|AxisEvents|InputAxisPitch AxisValue) (Variables|Default|GetTurn%20Rate) (Utilities|Time|GetWorldDeltaSeconds)) (.pitch _returnvalue)) (+ (* AxisValue (Variables|Default|GetTurn%20Rate) (Utilities|Time|GetWorldDeltaSeconds)) (.yaw _returnvalue))) false false))

(event Input|AxisEvents|InputAxisFirePrimaryWeapon
  (params (AxisValue :type Float%20%28single-precision%29))
  (bind _returnvalue (Transformation|GetActorTransform))
  ;[0 0.1479 1] Shooting Stuff
  (if (> AxisValue 0.0)
    (if (Variables|Default|GetFire%20Okay)
      (Game|SpawnActorfromClass "/Game/TRASH/Blueprints/BP_ProjectileActor1.BP_ProjectileActor1_C" (Math|Transform|MakeTransform (.location _returnvalue) (Transformation|GetWorldRotation (Variables|Default|GetStaticMesh)) (.scale _returnvalue)) "Undefined" 0 0)
      (Variables|Default|SetFire%20Okay false))))

(event Input|AxisEvents|InputAxisYaw
  (params (AxisValue :type Float%20%28single-precision%29))
  (bind _cameraspringoffsety (Variables|Default|GetCameraSpringOffsetY))
  ;[0 0.974 0.005356] Left/Right Camera Offset stuff
  (if (!= AxisValue 0.0)
    (Variables|/Script/Engine.SpringArmComponent|SetTargetArmLength _cameraspringoffsety (Math|Float|Clamp(Float) (+ (* AxisValue -6e+02 (Utilities|Time|GetWorldDeltaSeconds)) (Variables|/Script/Engine.SpringArmComponent|GetTargetArmLength _cameraspringoffsety)) (* (Variables|Default|GetCameraMaxMove) -1.0) (Variables|Default|GetCameraMaxMove)))
    (elif (> (Variables|/Script/Engine.SpringArmComponent|GetTargetArmLength (Variables|Default|GetCameraSpringOffsetY)) 0.0)
      (Variables|/Script/Engine.SpringArmComponent|SetTargetArmLength (Variables|Default|GetCameraSpringOffsetY) (+ (* -6e+02 (Utilities|Time|GetWorldDeltaSeconds)) (Variables|/Script/Engine.SpringArmComponent|GetTargetArmLength (Variables|Default|GetCameraSpringOffsetY))))
      (elif (< (Variables|/Script/Engine.SpringArmComponent|GetTargetArmLength (Variables|Default|GetCameraSpringOffsetY)) 0.0)
        (Variables|/Script/Engine.SpringArmComponent|SetTargetArmLength (Variables|Default|GetCameraSpringOffsetY) (+ (* 6e+02 (Utilities|Time|GetWorldDeltaSeconds)) (Variables|/Script/Engine.SpringArmComponent|GetTargetArmLength (Variables|Default|GetCameraSpringOffsetY))))))))

(event Input|AxisEvents|InputAxisPitch
  (params (AxisValue :type Float%20%28single-precision%29))
  (bind _cameraspringoffsetz (Variables|Default|GetCameraSpringOffsetZ))
  ;[0 0.974 0.005356] Up/Down Camera Offset stuff
  (if (!= AxisValue 0.0)
    (Variables|/Script/Engine.SpringArmComponent|SetTargetArmLength _cameraspringoffsetz (Math|Float|Clamp(Float) (+ (* AxisValue -6e+02 (Utilities|Time|GetWorldDeltaSeconds)) (Variables|/Script/Engine.SpringArmComponent|GetTargetArmLength _cameraspringoffsetz)) (* (Variables|Default|GetCameraMaxMove) -1.0) (Variables|Default|GetCameraMaxMove)))
    (elif (> (Variables|/Script/Engine.SpringArmComponent|GetTargetArmLength (Variables|Default|GetCameraSpringOffsetZ)) 0.0)
      (Variables|/Script/Engine.SpringArmComponent|SetTargetArmLength (Variables|Default|GetCameraSpringOffsetZ) (+ (* -6e+02 (Utilities|Time|GetWorldDeltaSeconds)) (Variables|/Script/Engine.SpringArmComponent|GetTargetArmLength (Variables|Default|GetCameraSpringOffsetZ))))
      (elif (< (Variables|/Script/Engine.SpringArmComponent|GetTargetArmLength (Variables|Default|GetCameraSpringOffsetZ)) 0.0)
        (Variables|/Script/Engine.SpringArmComponent|SetTargetArmLength (Variables|Default|GetCameraSpringOffsetZ) (+ (* 6e+02 (Utilities|Time|GetWorldDeltaSeconds)) (Variables|/Script/Engine.SpringArmComponent|GetTargetArmLength (Variables|Default|GetCameraSpringOffsetZ))))))))

(event Input|AxisEvents|InputAxisRoll
  (params (AxisValue :type Float%20%28single-precision%29))
  ;[1 1 1] Speed Control
  (if (!= AxisValue 0.0)
    (if (> AxisValue 0.0)
      (Variables|Default|SetMovement%20Speed 1e+04)
      (elif (< AxisValue 0.0)
        (Variables|Default|SetMovement%20Speed 1e+03)))
    (else
      (Variables|Default|SetMovement%20Speed 5e+03))))

(fn ConstructionScript)