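; Enemy gun turret that tracks the player pawn and is destroyed with an explosion when overlapped by a BP_ProjectileActor2.
; Every Tick it spawns an enemy projectile along the mesh's current rotation, with no fire-rate limit, then snaps the mesh's relative rotation toward the player.
; GetPlayerAimDirectoin supplies the look-at transform from the actor to the player.
; TurnToAngle, a partial rate-limited roll turn, is never called, and several disconnected aiming experiments remain.
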(event EventBeginPlay
  (Variables|Default|SetPlayerTarget (Game|Player|GetPlayerPawn 0)))

(event EventTick
  (params (DeltaSeconds :type Float%20%28single-precision%29))
  (bind _staticmesh (Variables|Default|GetStaticMesh))
  (bind _aimtransform (CallFunction|GetPlayerAimDirectoin))
  (Game|SpawnActorfromClass "/Game/Blueprints/BP_ProjectileEnemyActor2.BP_ProjectileEnemyActor2_C" (Math|Transform|MakeTransform (.location _aimtransform) (Transformation|GetWorldRotation _staticmesh) (.scale _aimtransform)) "Undefined" 0 0)
  (Transformation|SetRelativeRotation _staticmesh (.rotation _aimtransform) false false))

(event Collision|EventActorBeginOverlap
  (params (OtherActor :type Actor%20Object%20Reference))
  (Utilities|Casting|CastToBP_ProjectileActor2 OtherActor)
  (Actor|DestroyActor)
  (Effects|SpawnEmitteratLocation "/Game/StarterContent/Particles/P_Explosion.P_Explosion" (Transformation|GetActorLocation) "0, 0, 0" "10.000000,10.000000,10.000000"))

(fn ConstructionScript)

(fn GetPlayerAimDirectoin
  (bind _returnvalue (Transformation|GetActorTransform))
  (return (Math|Transform|MakeTransform (.location _returnvalue) (Math|Rotator|FindLookatRotation (.location (Transformation|GetActorTransform)) (.location (Transformation|GetActorTransform (Variables|Default|GetPlayerTarget)))) (.scale _returnvalue))))

(fn TurntoAngle
  (params (TargetDirection :type Rotator) (TurnRate :type Float%20%28double-precision%29))
  (bind _staticmesh (Variables|Default|GetStaticMesh))
  (bind _returnvalue (Transformation|GetWorldRotation _staticmesh))
  (if (> (Math|Float|Absolute(Float) (- (.roll TargetDirection) (.roll _returnvalue))) 1.8e+02)
    (if (> (.roll TargetDirection) 1.8e+02)
      (bind _output_get (Variables|Default|SetTempDir (- (.roll TargetDirection) 3.6e+02)))
      (if (> (Math|Float|Absolute(Float) (- _output_get (.roll _returnvalue))) TurnRate)
        (Transformation|AddLocalRotation _staticmesh (Math|Rotator|MakeRotator (* TurnRate (Utilities|Time|GetWorldDeltaSeconds)) 0.0 0.0) false false)))))