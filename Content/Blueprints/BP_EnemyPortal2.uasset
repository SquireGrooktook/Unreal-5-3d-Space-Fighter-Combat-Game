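; BP_EnemyPortal2 is an enemy portal that periodically spawns an actor while fewer than ten BP_Enemy_Fighter actors exist in the world.
; Tick counts down FighterSpawnTimer, clamped between zero and one second, and queries all fighters whenever it reaches zero.
; Below the cap, it resets the timer to FighterSpawnTimerMax and spawns at the portal's location and scale with zero rotation; the spawn node shows no class.
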(event EventBeginPlay
  (Variables|Default|SetFighterSpawnTimer (Variables|Default|GetFighterSpawnTimerMax)))

(event Collision|EventActorBeginOverlap
  (params (OtherActor :type Actor%20Object%20Reference)))

(event EventTick
  (params (DeltaSeconds :type Float%20%28single-precision%29))
  (bind _returnvalue (Transformation|GetActorTransform))
  (Variables|Default|SetFighterSpawnTimer (Math|Float|Clamp(Float) (- (Variables|Default|GetFighterSpawnTimer) (* (Utilities|Time|GetWorldDeltaSeconds) 1.0))))
  (if (not (> (Variables|Default|GetFighterSpawnTimer) 0.0))
    (bind _outactors (Actor|GetAllActorsOfClass "/Game/Blueprints/BP_Enemy_Fighter.BP_Enemy_Fighter_C"))
    (if (< (Utilities|Array|Length _outactors) 10)
      (Variables|Default|SetFighterSpawnTimer (Variables|Default|GetFighterSpawnTimerMax))
      (Game|SpawnActorfromClass "/Game/Blueprints/BP_Enemy_Fighter.BP_Enemy_Fighter_C" (Math|Transform|MakeTransform (.location _returnvalue) "0, 0,0.000000" (.scale _returnvalue)) "Undefined" 0 0))))

(fn ConstructionScript)