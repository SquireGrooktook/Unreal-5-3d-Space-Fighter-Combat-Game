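; BP_Missile1 is a missile actor that flies straight along its mesh's forward vector at a set Speed.
; Tick moves it by delta time without sweeping and counts down LifetimeTimer, destroying it silently on expiry.
; Overlapping a BP_LimitWall or BP_EnvironmentalObject, or having DestroyNow set, triggers an explosion emitter and sound before destruction.
; A cast to BP_FlagShip is left unconnected.
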(event EventBeginPlay)

(event Collision|EventActorBeginOverlap
  (params (OtherActor :type Actor%20Object%20Reference))
  (bind _returnvalue (Transformation|GetActorLocation))
  ;[0.4375 0 0] Collision Stuff
  (Utilities|Casting|CastToBP_LimitWall OtherActor
    (:then
      _)
    (:CastFailed
      (Utilities|Casting|CastToBP_EnvironmentalObject OtherActor)))
  (Effects|SpawnEmitteratLocation "/Game/StarterContent/Particles/P_Explosion.P_Explosion" _returnvalue "0, 0, 0" "10.000000,10.000000,10.000000")
  (Audio|PlaySoundatLocation "/Game/StarterContent/Audio/Explosion02.Explosion02" _returnvalue "0, 0, 0" 1.0 1.0 0.0 0 0 0 0)
  (Actor|DestroyActor))

(event EventTick
  (params (DeltaSeconds :type Float%20%28single-precision%29))
  (bind _returnvalue (Transformation|GetActorLocation))
  (bind _staticmesh (Variables|Default|GetStaticMesh))
  (bind _returnvalue_2 (Transformation|GetWorldTransform _staticmesh))
  (bind (_location _rotation _scale) (Math|Transform|BreakTransform _returnvalue_2))
  (Transformation|SetActorTransform (Math|Transform|MakeTransform (+ (* (Math|Vector|Normalize (Math|Vector|GetForwardVector _staticmesh)) (* (Utilities|Time|GetWorldDeltaSeconds) (Variables|Default|GetSpeed))) _location) (Transformation|GetWorldRotation (Variables|Default|GetStaticMesh)) _scale))
  (Variables|Default|SetLifetime_Timer (- (Variables|Default|GetLifetime_Timer) (* 1.0 (Utilities|Time|GetWorldDeltaSeconds))))
  (if (> (Variables|Default|GetLifetime_Timer) 0.0)
    (if (Variables|Default|GetDestroy_Now)
      ;[0.4375 0 0] Collision Stuff
      (Effects|SpawnEmitteratLocation "/Game/StarterContent/Particles/P_Explosion.P_Explosion" _returnvalue "0, 0, 0" "10.000000,10.000000,10.000000")
      (Audio|PlaySoundatLocation "/Game/StarterContent/Audio/Explosion02.Explosion02" _returnvalue "0, 0, 0" 1.0 1.0 0.0 0 0 0 0)
      (Actor|DestroyActor))
    (else
      (Actor|DestroyActor))))

(fn ConstructionScript)