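; BP_EnemyPortal is an enemy spawner that creates BP_Enemy_Fighter actors at its own location.
; A timer, randomized on BeginPlay and after each spawn, counts down on Tick but is clamped to 0–1, so its effective delay is at most about one second.
; At zero, it spawns a fighter only if the world's count of that class, found with GetAllActorsOfClass, is below MaxEnemySpawns.
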(event EventBeginPlay
  (Variables|Default|SetFighterSpawnTimer (Math|Random|RandomFloatinRange 2e+01 (Variables|Default|GetFighterSpawnTimerMax))))

(event Collision|EventActorBeginOverlap
  (params (OtherActor :type Actor%20Object%20Reference)))

(event EventTick
  (params (DeltaSeconds :type Float%20%28single-precision%29))
  (Variables|Default|SetFighterSpawnTimer (Math|Float|Clamp(Float) (- (Variables|Default|GetFighterSpawnTimer) (* (Utilities|Time|GetWorldDeltaSeconds) 1.0))))
  (if (not (> (Variables|Default|GetFighterSpawnTimer) 0.0))
    (bind _outactors (Actor|GetAllActorsOfClass "/Game/Blueprints/BP_Enemy_Fighter.BP_Enemy_Fighter_C"))
    (if (< (Utilities|Array|Length _outactors) (Variables|Default|GetMaxEnemySpawns))
      (Variables|Default|SetFighterSpawnTimer (Math|Random|RandomFloatinRange 2e+01 (Variables|Default|GetFighterSpawnTimerMax)))
      (Game|SpawnActorfromClass "/Game/Blueprints/BP_Enemy_Fighter.BP_Enemy_Fighter_C" (Math|Transform|MakeTransform (.location (Transformation|GetActorTransform)) "0, 0, 0" "1.000000,1.000000,1.000000") "Undefined" 0 0))))

(fn ConstructionScript)