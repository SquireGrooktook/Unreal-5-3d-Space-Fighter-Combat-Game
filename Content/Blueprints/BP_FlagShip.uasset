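; Enemy flagship actor that spawns fighters and is destroyed once missiles knock out its four weakpoints.
; A countdown in Tick spawns BP_Enemy_Fighter at the ship's location while fewer than five exist.
; Tick also polls overlaps with BP_Missile1: hits disable weakpoints and clear their meshes, while missiles touching the hull explode.
; With all weakpoints down, it explodes and destroys itself; player-collision effects and a final explosion sound are unconnected.
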(event EventBeginPlay
  (Variables|Default|SetFighterSpawnTimer (Variables|Default|GetFighterSpawnTimerMax)))

(event EventTick
  (params (DeltaSeconds :type Float%20%28single-precision%29))
  (bind _returnvalue (Transformation|GetActorTransform))
  (bind _staticmesh (Variables|Default|GetStaticMesh))
  (bind _overlappingactors (Collision|GetOverlappingActors _staticmesh "/Game/Blueprints/BP_Missile1.BP_Missile1_C" :!class /Script/Engine.PrimitiveComponent))
  (Variables|Default|SetFighterSpawnTimer (Math|Float|Clamp(Float) (- (Variables|Default|GetFighterSpawnTimer) (* (Utilities|Time|GetWorldDeltaSeconds) 1.0))))
  (if (> (Variables|Default|GetFighterSpawnTimer) 0.0)
    _
    (else
      (bind _outactors (Actor|GetAllActorsOfClass "/Game/Blueprints/BP_Enemy_Fighter.BP_Enemy_Fighter_C"))
      (if (< (Utilities|Array|Length _outactors) 5)
        (Variables|Default|SetFighterSpawnTimer (Variables|Default|GetFighterSpawnTimerMax))
        (Game|SpawnActorfromClass "/Game/Blueprints/BP_Enemy_Fighter.BP_Enemy_Fighter_C" (Math|Transform|MakeTransform (.location _returnvalue) "0, 0, 0" (.scale _returnvalue)) "Undefined" 0 0))))
  (if (Variables|Default|GetWeakpoint1_Active)
    (if (Utilities|Array|IsEmpty (Collision|GetOverlappingActors (Variables|Default|GetWeakpoint1) "/Game/Blueprints/BP_Missile1.BP_Missile1_C" :!class /Script/Engine.PrimitiveComponent))
      _
      (else
        (Effects|SpawnEmitteratLocation "/Game/StarterContent/Particles/P_Explosion.P_Explosion" (Transformation|GetWorldLocation (Variables|Default|GetWeakpoint1)) "0, 0, 0" "10.000000,10.000000,10.000000")
        (Variables|Default|SetWeakpoint1_Active false)
        (Components|StaticMesh|SetStaticMesh (Variables|Default|GetWeakpoint1) 0)
        (for _array_element (Collision|GetOverlappingActors (Variables|Default|GetStaticMesh) "/Game/Blueprints/BP_Missile1.BP_Missile1_C" :!class /Script/Engine.PrimitiveComponent)
          (Effects|SpawnEmitteratLocation "/Game/StarterContent/Particles/P_Explosion.P_Explosion" (Transformation|GetActorLocation _array_element) "0, 0, 0" "10.000000,10.000000,10.000000")
          (Actor|DestroyActor _array_element)
          (Audio|PlaySoundatLocation "/Game/explosion.explosion" (Transformation|GetActorLocation _array_element) "0, 0, 0" 1.0 1.0 0.0 0 0 0 0)))))
  (if (Variables|Default|GetWeakpoint2_Active)
    (if (Utilities|Array|IsEmpty (Collision|GetOverlappingActors (Variables|Default|GetWeakpoint2) "/Game/Blueprints/BP_Missile1.BP_Missile1_C" :!class /Script/Engine.PrimitiveComponent))
      _
      (else
        (Effects|SpawnEmitteratLocation "/Game/StarterContent/Particles/P_Explosion.P_Explosion" (Transformation|GetWorldLocation (Variables|Default|GetWeakpoint2)) "0, 0, 0" "10.000000,10.000000,10.000000")
        (Variables|Default|SetWeakpoint2_Active false)
        (Components|StaticMesh|SetStaticMesh (Variables|Default|GetWeakpoint2) 0)
        (for _array_element_2 (Collision|GetOverlappingActors (Variables|Default|GetStaticMesh) "/Game/Blueprints/BP_Missile1.BP_Missile1_C" :!class /Script/Engine.PrimitiveComponent)
          (Effects|SpawnEmitteratLocation "/Game/StarterContent/Particles/P_Explosion.P_Explosion" (Transformation|GetActorLocation _array_element_2) "0, 0, 0" "10.000000,10.000000,10.000000")
          (Actor|DestroyActor _array_element_2)
          (Audio|PlaySoundatLocation "/Game/explosion.explosion" (Transformation|GetActorLocation _array_element_2) "0, 0, 0" 1.0 1.0 0.0 0 0 0 0)))))
  (if (Variables|Default|GetWeakpoint3_Active)
    (if (Utilities|Array|IsEmpty (Collision|GetOverlappingActors (Variables|Default|GetWeakpoint3) "/Game/Blueprints/BP_Missile1.BP_Missile1_C" :!class /Script/Engine.PrimitiveComponent))
      _
      (else
        (Effects|SpawnEmitteratLocation "/Game/StarterContent/Particles/P_Explosion.P_Explosion" (Transformation|GetWorldLocation (Variables|Default|GetWeakpoint3)) "0, 0, 0" "10.000000,10.000000,10.000000")
        (Variables|Default|SetWeakpoint3_Active false)
        (Components|StaticMesh|SetStaticMesh (Variables|Default|GetWeakpoint3) 0)
        (for _array_element_3 (Collision|GetOverlappingActors (Variables|Default|GetStaticMesh) "/Game/Blueprints/BP_Missile1.BP_Missile1_C" :!class /Script/Engine.PrimitiveComponent)
          (Effects|SpawnEmitteratLocation "/Game/StarterContent/Particles/P_Explosion.P_Explosion" (Transformation|GetActorLocation _array_element_3) "0, 0, 0" "10.000000,10.000000,10.000000")
          (Actor|DestroyActor _array_element_3)
          (Audio|PlaySoundatLocation "/Game/explosion.explosion" (Transformation|GetActorLocation _array_element_3) "0, 0, 0" 1.0 1.0 0.0 0 0 0 0)))))
  (if (Variables|Default|GetWeakpoint4_Active)
    (if (Utilities|Array|IsEmpty (Collision|GetOverlappingActors (Variables|Default|GetWeakpoint4) "/Game/Blueprints/BP_Missile1.BP_Missile1_C" :!class /Script/Engine.PrimitiveComponent))
      _
      (else
        (Effects|SpawnEmitteratLocation "/Game/StarterContent/Particles/P_Explosion.P_Explosion" (Transformation|GetWorldLocation (Variables|Default|GetWeakpoint4)) "0, 0, 0" "10.000000,10.000000,10.000000")
        (Variables|Default|SetWeakpoint4_Active false)
        (Components|StaticMesh|SetStaticMesh (Variables|Default|GetWeakpoint4) 0)
        (for _array_element_4 (Collision|GetOverlappingActors (Variables|Default|GetStaticMesh) "/Game/Blueprints/BP_Missile1.BP_Missile1_C" :!class /Script/Engine.PrimitiveComponent)
          (Effects|SpawnEmitteratLocation "/Game/StarterContent/Particles/P_Explosion.P_Explosion" (Transformation|GetActorLocation _array_element_4) "0, 0, 0" "10.000000,10.000000,10.000000")
          (Actor|DestroyActor _array_element_4)
          (Audio|PlaySoundatLocation "/Game/explosion.explosion" (Transformation|GetActorLocation _array_element_4) "0, 0, 0" 1.0 1.0 0.0 0 0 0 0)))))
  (if (Math|Boolean|ORBoolean (Variables|Default|GetWeakpoint1_Active) (Variables|Default|GetWeakpoint2_Active) (Variables|Default|GetWeakpoint3_Active) (Variables|Default|GetWeakpoint4_Active))
    _
    (else
      (Variables|Default|SetDestroy_Okay true)))
  ;[1 1 1] Comment
  (if (Utilities|Array|IsEmpty _overlappingactors)
    _
    (else
      (for _array_element_5 _overlappingactors
        (Effects|SpawnEmitteratLocation "/Game/StarterContent/Particles/P_Explosion.P_Explosion" (Transformation|GetActorLocation _array_element_5) "0, 0, 0" "10.000000,10.000000,10.000000")
        (Audio|PlaySoundatLocation "/Game/StarterContent/Audio/Explosion02.Explosion02" (Transformation|GetActorLocation _array_element_5) "0, 0, 0" 1.0 1.0 0.0 0 0 0 0)
        (Actor|DestroyActor _array_element_5))))
  (if (Variables|Default|GetDestroy_Okay)
    (Effects|SpawnEmitteratLocation "/Game/StarterContent/Particles/P_Explosion.P_Explosion" (Transformation|GetWorldLocation (Variables|Default|GetStaticMesh)) "0, 0, 0" "200.000000,200.000000,200.000000")
    (Actor|DestroyActor)))

(fn ConstructionScript)