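; Enemy fighter that constantly flies along its mesh's forward vector and explodes when a BP_ProjectileActor2 overlaps it.
; Tick steers yaw and pitch at fixed speed toward random waypoints, whose height range extends below zero in lvl_Mission2.
; It turns aggressive when the player falls within an angular cone, regardless of distance, and reverts outside a wider one.
; While aggressive it tracks the player, firing BP_ProjectileEnemyActor2 on a cooldown when aligned.
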(event EventBeginPlay
  (Variables|Default|SetPlayerTarget (Game|Player|GetPlayerPawn 0))
  (bind _newparam (CallFunction|PickRandomLocation))
  (Variables|Default|SetSearchTransform _newparam)
  (bind _returnvalue (Game|GetCurrentLevelName true))
  (if (Utilities|Enum|Equal(Enum) _returnvalue "lvl_Mission2")
    (Variables|Default|SetZ_Random_Lock -6e+04)
    (else
      (Variables|Default|SetZ_Random_Lock 0.0))))

(event EventTick
  (params (DeltaSeconds :type Float%20%28single-precision%29))
  (bind _returnvalue (Transformation|GetActorTransform))
  (bind _returnvalue_2 (Transformation|GetActorTransform))
  (bind _staticmesh (Variables|Default|GetStaticMesh))
  (bind _returnvalue_3 (Transformation|GetWorldTransform _staticmesh))
  (bind (_location _rotation _scale) (Math|Transform|BreakTransform _returnvalue_3))
  (Transformation|SetActorTransform (Math|Transform|MakeTransform (+ (* (Math|Vector|Normalize (Math|Vector|GetForwardVector _staticmesh)) (* (Utilities|Time|GetWorldDeltaSeconds) (Variables|Default|GetMovement%20Speed))) _location) "0, 0, 0" _scale))
  (Variables|Default|SetShotCooldown (Math|Float|Clamp(Float) (- (Variables|Default|GetShotCooldown) (* (Utilities|Time|GetWorldDeltaSeconds) 1.0)) 0.0 (Variables|Default|GetShotCoolDownAmount)))
  (if (Variables|Default|GetAggro)
    (if (Utilities|IsValid (Variables|Default|GetPlayerTarget))
      (bind _aimtransform (CallFunction|GetPlayerAimDirectoin))
      (bind _aimokay (CallFunction|CheckAim (.pitch (.rotation _aimtransform)) (.yaw (.rotation _aimtransform)) 1e+02))
      (if _aimokay
        (CallFunction|RotateAxisZ2 (.yaw (.rotation _aimtransform)))
        (CallFunction|RotateAxisY (.pitch (.rotation _aimtransform)))
        (bind _aimokay_2 (CallFunction|CheckAim (.pitch (.rotation _aimtransform)) (.yaw (.rotation _aimtransform)) (Variables|Default|GetAimTolerance)))
        (if _aimokay_2
          (if (> (Variables|Default|GetShotCooldown) 0.0)
            _
            (else
              (Game|SpawnActorfromClass "/Game/Blueprints/BP_ProjectileEnemyActor2.BP_ProjectileEnemyActor2_C" (Math|Transform|MakeTransform (.location _returnvalue) (Transformation|GetWorldRotation (Variables|Default|GetStaticMesh)) (.scale _returnvalue)) "Undefined" 0 0)
              (Variables|Default|SetShotCooldown (Variables|Default|GetShotCoolDownAmount)))))
        (else
          (Variables|Default|SetAggro false))))
    (else
      (bind _newparam (CallFunction|GetTotalDistance))
      (if (> _newparam 3e+01)
        (CallFunction|RotateAxisZ2 (.yaw (.rotation (Math|Transform|MakeTransform (.location _returnvalue_2) (Math|Rotator|FindLookatRotation (.location (Transformation|GetActorTransform)) (.location (Variables|Default|GetSearchTransform))) (.scale _returnvalue_2)))))
        (CallFunction|RotateAxisY (.pitch (.rotation (Math|Transform|MakeTransform (.location _returnvalue_2) (Math|Rotator|FindLookatRotation (.location (Transformation|GetActorTransform)) (.location (Variables|Default|GetSearchTransform))) (.scale _returnvalue_2)))))
        (if (Utilities|IsValid (Variables|Default|GetPlayerTarget))
          (bind _aimtransform_2 (CallFunction|GetPlayerAimDirectoin))
          (bind _aimokay_3 (CallFunction|CheckAim (.pitch (.rotation _aimtransform_2)) (.yaw (.rotation _aimtransform_2)) 5e+01))
          (if _aimokay_3
            (Variables|Default|SetAggro true)))
        (else
          (bind _newparam_2 (CallFunction|PickRandomLocation))
          (Variables|Default|SetSearchTransform _newparam_2)))))
  (if (Variables|Default|GetDestroy_Safety_Lock)
    (Effects|SpawnEmitteratLocation "/Game/StarterContent/Particles/P_Explosion.P_Explosion" (Transformation|GetActorLocation) "0, 0, 0" "10.000000,10.000000,10.000000")
    (Actor|DestroyActor)))

(event Collision|EventActorBeginOverlap
  (params (OtherActor :type Actor%20Object%20Reference))
  (Utilities|Casting|CastToBP_ProjectileActor2 OtherActor)
  (Variables|Default|SetDestroy_Safety_Lock true))

(fn ConstructionScript)

(fn GetPlayerAimDirectoin
  (bind _returnvalue (Transformation|GetActorTransform))
  (return (Math|Transform|MakeTransform (.location _returnvalue) (Math|Rotator|FindLookatRotation (.location (Transformation|GetActorTransform)) (.location (Transformation|GetActorTransform (Variables|Default|GetPlayerTarget)))) (.scale _returnvalue))))

(fn PerformRotationZ
  (params (Dir :type Float%20%28double-precision%29))
  (Transformation|AddLocalRotation (Variables|Default|GetStaticMesh) (Math|Rotator|MakeRotator 0.0 0.0 (* (Variables|Default|GetRotationSpeed) (Utilities|Time|GetWorldDeltaSeconds) Dir)) false false))

(fn RotateAxisZ2
  (params (TargetRotation :type Float%20%28double-precision%29))
  (bind _staticmesh (Variables|Default|GetStaticMesh))
  (bind _returnvalue (Transformation|GetWorldRotation _staticmesh))
  (bind _returnvalue_2 (- (.yaw _returnvalue) TargetRotation))
  (bind _returnvalue_3 (Math|Float|Absolute(Float) _returnvalue_2))
  (bind _returnvalue_4 (> _returnvalue_3 1.8e+02))
  (Variables|Default|SetTempDir 0.0)
  (Variables|Default|SetFinalDirectionDir 0.0)
  (if (< (Math|Float|Absolute(Float) (- (.yaw _returnvalue) TargetRotation)) 1.0)
    (Transformation|SetRelativeRotation (Variables|Default|GetStaticMesh) (Math|Rotator|MakeRotator (.roll _returnvalue) (.pitch _returnvalue) TargetRotation) false false)
    (else
      (if (> (.yaw _returnvalue) TargetRotation)
        (if _returnvalue_4
          (Variables|Default|SetFinalDirectionDir 1.0)
          (else
            (Variables|Default|SetFinalDirectionDir -1.0)))
        (elif _returnvalue_4
          (bind _output_get (Variables|Default|SetFinalDirectionDir -1.0))
          (else
            (Variables|Default|SetFinalDirectionDir 1.0))))
      (CallFunction|PerformRotationZ _output_get))))

(fn RotateAxisY
  (params (TargetRotation :type Float%20%28double-precision%29))
  (bind _staticmesh (Variables|Default|GetStaticMesh))
  (bind _returnvalue (Transformation|GetWorldRotation _staticmesh))
  (bind _returnvalue_2 (- (.pitch _returnvalue) TargetRotation))
  (bind _returnvalue_3 (Math|Float|Absolute(Float) _returnvalue_2))
  (bind _returnvalue_4 (> _returnvalue_3 1.8e+02))
  (Variables|Default|SetTempDir 0.0)
  (Variables|Default|SetFinalDirectionDir 0.0)
  (if (< (Math|Float|Absolute(Float) (- (.pitch _returnvalue) TargetRotation)) 1.0)
    (Transformation|SetRelativeRotation (Variables|Default|GetStaticMesh) (Math|Rotator|MakeRotator (.roll _returnvalue) TargetRotation (.yaw _returnvalue)) false false)
    (else
      (if (> (.pitch _returnvalue) TargetRotation)
        (if _returnvalue_4
          (Variables|Default|SetFinalDirectionDir 1.0)
          (else
            (bind _output_get (Variables|Default|SetFinalDirectionDir -1.0))))
        (elif _returnvalue_4
          (Variables|Default|SetFinalDirectionDir -1.0)
          (else
            (Variables|Default|SetFinalDirectionDir 1.0))))
      (CallFunction|PerformRotationY _output_get))))

(fn PerformRotationY
  (params (Dir :type Float%20%28double-precision%29))
  (Transformation|AddLocalRotation (Variables|Default|GetStaticMesh) (Math|Rotator|MakeRotator 0.0 (* (Variables|Default|GetRotationSpeed) (Utilities|Time|GetWorldDeltaSeconds) Dir) 0.0) false false))

(fn CheckAim
  (params (TargetRotationY :type Float%20%28double-precision%29) (TargetRotationZ :type Float%20%28double-precision%29) (DegreesToCheck :type Float%20%28double-precision%29))
  (bind _staticmesh (Variables|Default|GetStaticMesh))
  (bind _returnvalue (Transformation|GetWorldRotation _staticmesh))
  (return (and (< (Math|Float|Absolute(Float) (- TargetRotationY (.pitch _returnvalue))) DegreesToCheck) (< (Math|Float|Absolute(Float) (- TargetRotationZ (.yaw _returnvalue))) DegreesToCheck))))

(fn PickRandomLocation
  (return (Math|Transform|MakeTransform (Math|Vector|MakeVector (Math|Random|RandomFloatinRange -6e+03 1.2e+03) (Math|Random|RandomFloatinRange -6e+04 6e+04) (Math|Random|RandomFloatinRange (Variables|Default|GetZ_Random_Lock) 6e+04)) "0, 0, 0" "1.000000,1.000000,1.000000")))

(fn GetTotalDistance
  (return (Math|Vector|Distance(Vector) (Transformation|GetWorldLocation (Variables|Default|GetStaticMesh)) (.location (Variables|Default|GetSearchTransform)))))